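; Base Blueprint for a destructible object that takes hits from NonDestructableObject actors.
; When its Destructible component is hit by such an actor with positive momentum (speed times Weight), it loses one hitpoint.
; A qualifying hit that arrives with Hitpoints already below one applies damage to the component at the hitting actor's location, along the hit's normal impulse.
; Leftover debug prints mark the hit and failed checks.
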(event OnComponentHit(Destructible)
  (params (HitComponent :type Primitive%20Component%20Object%20Reference) (OtherActor :type Actor%20Object%20Reference) (OtherComp :type Primitive%20Component%20Object%20Reference) (NormalImpulse :type Vector :default "0, 0, 0") (Hit :type Hit%20Result%20Structure%20%28by%20ref%29))
  (Development|PrintString "2343241")
  (if (Utilities|ClassIsChildOf (Utilities|GetClass OtherActor) "/Game/Blueprints/Objects/NonDestructableObject.NonDestructableObject_C")
    (bind _asnon_destructable_object (Utilities|Casting|CastToNonDestructableObject OtherActor)
      (:then
        (if (> (* (Math|Vector|VectorLength (Transformation|GetVelocity OtherActor)) (Variables|/Game/Blueprints/Objects/NonDestructableObject.NonDestructableObject_C|GetWeight _asnon_destructable_object)) 0.0)
          (if (< (Variables|Default|GetHitpoints) 1.0)
            (Class|DestructibleComponent|ApplyDamage (Variables|Default|GetDestructible) 1.0 (Transformation|GetActorLocation OtherActor) NormalImpulse 0.0)
            (else
              (bind _result (Math|Float|DecrementFloat (Variables|Default|GetHitpoints))
                (:%20%20
                  (Variables|Default|SetHitpoints _result)))))
          (else
            (Development|PrintString "Hello"))))
      (:CastFailed
        (Development|PrintString "Failed cast")))
    (else
      (Development|PrintString "no"))))

(event EventBeginPlay
  (|CallParentFunction) ; This node is disabled and will not be called.\nDrag off pins to build functionality.
)

(event Collision|EventActorBeginOverlap
  (params (OtherActor :type Actor%20Object%20Reference))
  (|CallParentFunction OtherActor) ; This node is disabled and will not be called.\nDrag off pins to build functionality.
)

(event EventTick
  (params (DeltaSeconds :type Float%20%28single-precision%29))
  (|CallParentFunction DeltaSeconds) ; This node is disabled and will not be called.\nDrag off pins to build functionality.
)

(fn ConstructionScript
  (|CallParentFunction))